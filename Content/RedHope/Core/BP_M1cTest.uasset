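; BP_M1cTest is an unattended test actor that exercises the RedHope world-pressure milestone, a storm at sol 2 and a flare at sol 4.
; On BeginPlay it issues RH console commands to speed time, dig, and build a small power and storage base.
; A timed Delay chain then switches to high-speed era mode, expecting auto-drops before each event, and logs status and fleet snapshots around them.
; Printed expectations describe the intended results, with no automated assertions.
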(event `self.ReceiveBeginPlay`
  (`KismetSystemLibrary.Delay` 3.0)
  (`KismetSystemLibrary.ExecuteConsoleCommand` "RH.SetSpeed 8" null)
  (`KismetSystemLibrary.PrintString` "RH M1C TEST: world pressure - storm at sol 2, flare at sol 4. Hands off.")
  (`KismetSystemLibrary.ExecuteConsoleCommand` "RH.Dig Regolith_A" null)
  (`KismetSystemLibrary.ExecuteConsoleCommand` "RH.Build ChargePad 0 -14" null)
  (`KismetSystemLibrary.ExecuteConsoleCommand` "RH.Build SolarArray -12 -15" null)
  (`KismetSystemLibrary.ExecuteConsoleCommand` "RH.Build SolarArray -12 -5" null)
  (`KismetSystemLibrary.ExecuteConsoleCommand` "RH.Build SolarArray -12 5" null)
  (`KismetSystemLibrary.ExecuteConsoleCommand` "RH.Build SolarArray -12 15" null)
  (`KismetSystemLibrary.ExecuteConsoleCommand` "RH.Build BatteryBank -20 10" null)
  (`KismetSystemLibrary.ExecuteConsoleCommand` "RH.Build Stockpile 10 8" null)
  (`KismetSystemLibrary.Delay` 150.0)
  (`KismetSystemLibrary.ExecuteConsoleCommand` "RH.Status" null)
  (`KismetSystemLibrary.ExecuteConsoleCommand` "RH.Fleet" null)
  (`KismetSystemLibrary.Delay` 60.0)
  (`KismetSystemLibrary.PrintString` "RH M1C: engaging era mode - must AUTO-DROP before the sol-2 storm onset")
  (`KismetSystemLibrary.ExecuteConsoleCommand` "RH.SetSpeed 60" null)
  (`KismetSystemLibrary.Delay` 30.0)
  (`KismetSystemLibrary.ExecuteConsoleCommand` "RH.Status" null)
  (`KismetSystemLibrary.Delay` 75.0)
  (`KismetSystemLibrary.PrintString` "RH M1C: mid-storm status - expect gen collapsed, SHED, event line")
  (`KismetSystemLibrary.ExecuteConsoleCommand` "RH.Status" null)
  (`KismetSystemLibrary.Delay` 90.0)
  (`KismetSystemLibrary.PrintString` "RH M1C: storm over - re-engaging era; must auto-drop again before the sol-4 flare")
  (`KismetSystemLibrary.ExecuteConsoleCommand` "RH.Status" null)
  (`KismetSystemLibrary.ExecuteConsoleCommand` "RH.Fleet" null)
  (`KismetSystemLibrary.ExecuteConsoleCommand` "RH.SetSpeed 60" null)
  (`KismetSystemLibrary.Delay` 45.0)
  (`KismetSystemLibrary.ExecuteConsoleCommand` "RH.Status" null)
  (`KismetSystemLibrary.ExecuteConsoleCommand` "RH.Fleet" null)
  (`KismetSystemLibrary.Delay` 45.0)
  (`KismetSystemLibrary.PrintString` "RH M1C: flare should have passed - wear delta vs pre-flare snapshot is the tax")
  (`KismetSystemLibrary.ExecuteConsoleCommand` "RH.Status" null)
  (`KismetSystemLibrary.ExecuteConsoleCommand` "RH.Fleet" null)
  (`KismetSystemLibrary.PrintString` "RH_M1C_DONE"))

(fn `UserConstructionScript`)