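; BP_M0aTest is a scripted smoke-test actor for the RedHope game's console-driven build commands.
; On BeginPlay it raises game speed, then uses timed delays to issue RH.Build commands for a pylon, solar array and stockpile at set positions.
; RH.Status is queried between steps, and a completion marker string prints at the end.
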(event `self.ReceiveBeginPlay`
  (`KismetSystemLibrary.Delay` 3.0)
  (`KismetSystemLibrary.ExecuteConsoleCommand` "RH.SetSpeed 8" null)
  (`KismetSystemLibrary.ExecuteConsoleCommand` "RH.Status" null)
  (`KismetSystemLibrary.Delay` 1.0)
  (`KismetSystemLibrary.ExecuteConsoleCommand` "RH.Build Pylon 25 0" null)
  (`KismetSystemLibrary.Delay` 2.0)
  (`KismetSystemLibrary.ExecuteConsoleCommand` "RH.Status" null)
  (`KismetSystemLibrary.Delay` 6.0)
  (`KismetSystemLibrary.ExecuteConsoleCommand` "RH.Status" null)
  (`KismetSystemLibrary.ExecuteConsoleCommand` "RH.Build SolarArray 50 0" null)
  (`KismetSystemLibrary.Delay` 8.0)
  (`KismetSystemLibrary.ExecuteConsoleCommand` "RH.Status" null)
  (`KismetSystemLibrary.ExecuteConsoleCommand` "RH.Build Stockpile 200 0" null)
  (`KismetSystemLibrary.Delay` 8.0)
  (`KismetSystemLibrary.ExecuteConsoleCommand` "RH.Status" null)
  (`KismetSystemLibrary.Delay` 30.0)
  (`KismetSystemLibrary.ExecuteConsoleCommand` "RH.Status" null)
  (`KismetSystemLibrary.PrintString` "RHM0A_DONE"))

(fn `UserConstructionScript`)