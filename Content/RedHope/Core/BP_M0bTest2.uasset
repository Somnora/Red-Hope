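; BP_M0bTest2 is a scripted smoke test actor for RedHope that drives the game through RH console commands on BeginPlay.
; After a short delay it sets lag and speed, starts regolith digging, and builds solar arrays, a battery bank and a forge.
; It then logs RH.Status at timed intervals and prints a completion marker when the sequence finishes.
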(event `self.ReceiveBeginPlay`
  (`KismetSystemLibrary.Delay` 3.0)
  (`KismetSystemLibrary.ExecuteConsoleCommand` "RH.Lag 5" null)
  (`KismetSystemLibrary.ExecuteConsoleCommand` "RH.SetSpeed 8" null)
  (`KismetSystemLibrary.ExecuteConsoleCommand` "RH.Dig Regolith_A" null)
  (`KismetSystemLibrary.ExecuteConsoleCommand` "RH.Build SolarArray 10 -8" null)
  (`KismetSystemLibrary.Delay` 2.0)
  (`KismetSystemLibrary.ExecuteConsoleCommand` "RH.Build SolarArray 10 -2" null)
  (`KismetSystemLibrary.ExecuteConsoleCommand` "RH.Build BatteryBank 14 -8" null)
  (`KismetSystemLibrary.ExecuteConsoleCommand` "RH.Build Forge -15 10" null)
  (`KismetSystemLibrary.Delay` 15.0)
  (`KismetSystemLibrary.ExecuteConsoleCommand` "RH.Status" null)
  (`KismetSystemLibrary.Delay` 20.0)
  (`KismetSystemLibrary.ExecuteConsoleCommand` "RH.Status" null)
  (`KismetSystemLibrary.Delay` 20.0)
  (`KismetSystemLibrary.ExecuteConsoleCommand` "RH.Status" null)
  (`KismetSystemLibrary.Delay` 20.0)
  (`KismetSystemLibrary.ExecuteConsoleCommand` "RH.Status" null)
  (`KismetSystemLibrary.Delay` 15.0)
  (`KismetSystemLibrary.ExecuteConsoleCommand` "RH.Status" null)
  (`KismetSystemLibrary.Delay` 15.0)
  (`KismetSystemLibrary.ExecuteConsoleCommand` "RH.Status" null)
  (`KismetSystemLibrary.PrintString` "RHM0B2_DONE"))

(fn `UserConstructionScript`)