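; BP_DemoReel is a scripted demo driver that plays a RedHope base-building and launch sequence hands-free for recording.
; BeginPlay runs one linear chain of Delays and RH.* console commands: it speeds up the game, digs, then builds power, industry, pylons and ice/water facilities in timed stages.
; It then repeats a manifest-and-launch cycle three times, logging status throughout and printing progress and completion messages.
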(event `self.ReceiveBeginPlay`
  (`KismetSystemLibrary.Delay` 3.0)
  (`KismetSystemLibrary.ExecuteConsoleCommand` "RH.SetSpeed 8" null)
  (`KismetSystemLibrary.ExecuteConsoleCommand` "RH.Status" null)
  (`KismetSystemLibrary.ExecuteConsoleCommand` "RH.Dig Regolith_A" null)
  (`KismetSystemLibrary.ExecuteConsoleCommand` "RH.Build ChargePad 0 -14" null)
  (`KismetSystemLibrary.ExecuteConsoleCommand` "RH.Build SolarArray -12 -15" null)
  (`KismetSystemLibrary.ExecuteConsoleCommand` "RH.Build SolarArray -12 -5" null)
  (`KismetSystemLibrary.ExecuteConsoleCommand` "RH.Build SolarArray -12 5" null)
  (`KismetSystemLibrary.ExecuteConsoleCommand` "RH.Build SolarArray -12 15" null)
  (`KismetSystemLibrary.ExecuteConsoleCommand` "RH.Build BatteryBank -20 10" null)
  (`KismetSystemLibrary.ExecuteConsoleCommand` "RH.Build Forge 16 -14" null)
  (`KismetSystemLibrary.ExecuteConsoleCommand` "RH.Build Pylon 55 55" null)
  (`KismetSystemLibrary.Delay` 150.0)
  (`KismetSystemLibrary.ExecuteConsoleCommand` "RH.Status" null)
  (`KismetSystemLibrary.ExecuteConsoleCommand` "RH.Build Pylon 110 110" null)
  (`KismetSystemLibrary.Delay` 90.0)
  (`KismetSystemLibrary.ExecuteConsoleCommand` "RH.Status" null)
  (`KismetSystemLibrary.ExecuteConsoleCommand` "RH.Build IceDrill 130 130" null)
  (`KismetSystemLibrary.ExecuteConsoleCommand` "RH.Build WaterPlant 118 122" null)
  (`KismetSystemLibrary.Delay` 170.0)
  (`KismetSystemLibrary.ExecuteConsoleCommand` "RH.Status" null)
  (`KismetSystemLibrary.ExecuteConsoleCommand` "RH.Build Electrolyzer 14 20" null)
  (`KismetSystemLibrary.Delay` 200.0)
  (`KismetSystemLibrary.ExecuteConsoleCommand` "RH.Status" null)
  (`KismetSystemLibrary.ExecuteConsoleCommand` "RH.Manifest SolarPack" null)
  (`KismetSystemLibrary.ExecuteConsoleCommand` "RH.Manifest BatteryPack" null)
  (`KismetSystemLibrary.ExecuteConsoleCommand` "RH.Manifest PartsCrate" null)
  (`KismetSystemLibrary.ExecuteConsoleCommand` "RH.Manifest ComputeCore" null)
  (`KismetSystemLibrary.ExecuteConsoleCommand` "RH.Launch" null)
  (`KismetSystemLibrary.ExecuteConsoleCommand` "RH.Status" null)
  (`KismetSystemLibrary.Delay` 120.0)
  (`KismetSystemLibrary.ExecuteConsoleCommand` "RH.Manifest SolarPack" null)
  (`KismetSystemLibrary.ExecuteConsoleCommand` "RH.Manifest BatteryPack" null)
  (`KismetSystemLibrary.ExecuteConsoleCommand` "RH.Manifest PartsCrate" null)
  (`KismetSystemLibrary.ExecuteConsoleCommand` "RH.Manifest ComputeCore" null)
  (`KismetSystemLibrary.ExecuteConsoleCommand` "RH.Launch" null)
  (`KismetSystemLibrary.ExecuteConsoleCommand` "RH.Status" null)
  (`KismetSystemLibrary.Delay` 120.0)
  (`KismetSystemLibrary.ExecuteConsoleCommand` "RH.Manifest SolarPack" null)
  (`KismetSystemLibrary.ExecuteConsoleCommand` "RH.Manifest BatteryPack" null)
  (`KismetSystemLibrary.ExecuteConsoleCommand` "RH.Manifest PartsCrate" null)
  (`KismetSystemLibrary.ExecuteConsoleCommand` "RH.Manifest ComputeCore" null)
  (`KismetSystemLibrary.ExecuteConsoleCommand` "RH.Launch" null)
  (`KismetSystemLibrary.ExecuteConsoleCommand` "RH.Status" null)
  (`KismetSystemLibrary.PrintString` "RH DEMO: quota arc running - after the LAUNCHED toast the ship lands ~7 min later at 8x. Safe to stop recording after launch.")
  (`KismetSystemLibrary.Delay` 450.0)
  (`KismetSystemLibrary.ExecuteConsoleCommand` "RH.Status" null)
  (`KismetSystemLibrary.Delay` 240.0)
  (`KismetSystemLibrary.ExecuteConsoleCommand` "RH.Status" null)
  (`KismetSystemLibrary.PrintString` "RH_DEMO_DONE"))

(fn `UserConstructionScript`)