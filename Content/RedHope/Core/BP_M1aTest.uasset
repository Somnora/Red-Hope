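; BP_M1aTest is a scripted test actor that exercises RedHope's dig, build, time-speed and save/load features.
; On BeginPlay it runs a timed chain of RH console commands separated by delays, starting a regolith dig and placing base structures.
; It saves and reloads two named slots, switches simulation speed and issues status reports at checkpoints.
; It prints RHM1A_DONE when the sequence finishes.
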(event `self.ReceiveBeginPlay`
  (`KismetSystemLibrary.Delay` 2.0)
  (`KismetSystemLibrary.ExecuteConsoleCommand` "RH.SetSpeed 8" null)
  (`KismetSystemLibrary.ExecuteConsoleCommand` "RH.Dig Regolith_A" null)
  (`KismetSystemLibrary.ExecuteConsoleCommand` "RH.Build SolarArray -12 -8" null)
  (`KismetSystemLibrary.ExecuteConsoleCommand` "RH.Build SolarArray -12 0" null)
  (`KismetSystemLibrary.ExecuteConsoleCommand` "RH.Build BatteryBank -20 8" null)
  (`KismetSystemLibrary.ExecuteConsoleCommand` "RH.Build ChargePad 0 -14" null)
  (`KismetSystemLibrary.ExecuteConsoleCommand` "RH.Build Forge 16 -14" null)
  (`KismetSystemLibrary.Delay` 98.0)
  (`KismetSystemLibrary.ExecuteConsoleCommand` "RH.Build Stockpile 10 8" null)
  (`KismetSystemLibrary.Delay` 48.0)
  (`KismetSystemLibrary.ExecuteConsoleCommand` "RH.Status" null)
  (`KismetSystemLibrary.ExecuteConsoleCommand` "RH.Save siteA" null)
  (`KismetSystemLibrary.Delay` 50.0)
  (`KismetSystemLibrary.ExecuteConsoleCommand` "RH.Status" null)
  (`KismetSystemLibrary.ExecuteConsoleCommand` "RH.Load siteA" null)
  (`KismetSystemLibrary.ExecuteConsoleCommand` "RH.SetSpeed 8" null)
  (`KismetSystemLibrary.Delay` 50.0)
  (`KismetSystemLibrary.ExecuteConsoleCommand` "RH.Status" null)
  (`KismetSystemLibrary.ExecuteConsoleCommand` "RH.SetSpeed 60" null)
  (`KismetSystemLibrary.Delay` 8.0)
  (`KismetSystemLibrary.ExecuteConsoleCommand` "RH.Status" null)
  (`KismetSystemLibrary.ExecuteConsoleCommand` "RH.SetSpeed 8" null)
  (`KismetSystemLibrary.Delay` 144.0)
  (`KismetSystemLibrary.ExecuteConsoleCommand` "RH.Status" null)
  (`KismetSystemLibrary.ExecuteConsoleCommand` "RH.Save clean" null)
  (`KismetSystemLibrary.Delay` 150.0)
  (`KismetSystemLibrary.ExecuteConsoleCommand` "RH.Status" null)
  (`KismetSystemLibrary.ExecuteConsoleCommand` "RH.Load clean" null)
  (`KismetSystemLibrary.ExecuteConsoleCommand` "RH.SetSpeed 60" null)
  (`KismetSystemLibrary.Delay` 20.0)
  (`KismetSystemLibrary.ExecuteConsoleCommand` "RH.Status" null)
  (`KismetSystemLibrary.ExecuteConsoleCommand` "RH.SetSpeed 8" null)
  (`KismetSystemLibrary.Delay` 5.0)
  (`KismetSystemLibrary.ExecuteConsoleCommand` "RH.Status" null)
  (`KismetSystemLibrary.PrintString` "RHM1A_DONE"))

(fn `UserConstructionScript`)