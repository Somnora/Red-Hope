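; BP_StressDriver is an automated stress-test actor that benchmarks RedHope under rising dummy counts and game speeds.
; On BeginPlay it runs a fixed, Delay-spaced sequence of RH console commands: a baseline benchmark, then labeled runs after each dummy spawn at normal and accelerated speed.
; It also takes a high-resolution screenshot before the heaviest run, then resets speed and prints a completion marker.
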(event `self.ReceiveBeginPlay`
  (`KismetSystemLibrary.Delay` 5.0)
  (`KismetSystemLibrary.ExecuteConsoleCommand` "RH.Benchmark base0 10" null)
  (`KismetSystemLibrary.Delay` 12.0)
  (`KismetSystemLibrary.ExecuteConsoleCommand` "RH.SpawnDummies 200 300" null)
  (`KismetSystemLibrary.Delay` 3.0)
  (`KismetSystemLibrary.ExecuteConsoleCommand` "RH.Benchmark a200x1 12" null)
  (`KismetSystemLibrary.Delay` 14.0)
  (`KismetSystemLibrary.ExecuteConsoleCommand` "RH.SetSpeed 8" null)
  (`KismetSystemLibrary.Delay` 2.0)
  (`KismetSystemLibrary.ExecuteConsoleCommand` "RH.Benchmark a200x8 12" null)
  (`KismetSystemLibrary.Delay` 14.0)
  (`KismetSystemLibrary.ExecuteConsoleCommand` "RH.SetSpeed 1" null)
  (`KismetSystemLibrary.ExecuteConsoleCommand` "RH.SpawnDummies 300 300" null)
  (`KismetSystemLibrary.Delay` 3.0)
  (`KismetSystemLibrary.ExecuteConsoleCommand` "RH.Benchmark a500x1 12" null)
  (`KismetSystemLibrary.Delay` 14.0)
  (`KismetSystemLibrary.ExecuteConsoleCommand` "RH.SetSpeed 8" null)
  (`KismetSystemLibrary.Delay` 2.0)
  (`KismetSystemLibrary.ExecuteConsoleCommand` "HighResShot 1920x1080" null)
  (`KismetSystemLibrary.Delay` 1.0)
  (`KismetSystemLibrary.ExecuteConsoleCommand` "RH.Benchmark a500x8 12" null)
  (`KismetSystemLibrary.Delay` 14.0)
  (`KismetSystemLibrary.ExecuteConsoleCommand` "RH.SetSpeed 1" null)
  (`KismetSystemLibrary.PrintString` "RHSTRESS_SEQUENCE_DONE"))

(fn `UserConstructionScript`)