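; BP_VaultDemo is a hands-off scripted demo of building the first livable underground floor in the RedHope colony game.
; On BeginPlay it runs a timed chain of RH console commands: showcase setup and stock, shaft boring, excavation, air filter construction and habitat commands during pressurization.
; Delays pace each step, on-screen prints narrate it, and the game speed is repeatedly re-applied while it waits.
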(event `self.ReceiveBeginPlay`
  (`KismetSystemLibrary.Delay` 5.0)
  (`KismetSystemLibrary.PrintString` "VAULT DEMO: hands off - watch. I will build the first livable floor. A test dust storm hits at sol 2: speed snaps to 1x (batten down), then I re-speed.")
  (`KismetSystemLibrary.ExecuteConsoleCommand` "RH.Showcase" null)
  (`KismetSystemLibrary.ExecuteConsoleCommand` "RH.AddStock Oxygen 500" null)
  (`KismetSystemLibrary.ExecuteConsoleCommand` "RH.AddStock Hydrogen 20" null)
  (`KismetSystemLibrary.PrintString` "STEP 1 - BORE: the Borer never runs by itself, it works ORDERS. Ordering the shaft one floor down. (Console: RH.Bore 1 - a deck Bore button lands next compile.)")
  (`KismetSystemLibrary.ExecuteConsoleCommand` "RH.Bore 1" null)
  (`KismetSystemLibrary.ExecuteConsoleCommand` "RH.SetSpeed 8" null)
  (`KismetSystemLibrary.Delay` 85.0)
  (`KismetSystemLibrary.PrintString` "STEP 2 - EXCAVATE: shaft reached -1. Ordering 4 cells carved (by hand: Excavate button, then click-drag on the floor). Dropping the elevator to -1 - watch tiles appear.")
  (`KismetSystemLibrary.ExecuteConsoleCommand` "RH.Excavate -1 4" null)
  (`KismetSystemLibrary.ExecuteConsoleCommand` "RH.Floor -1" null)
  (`KismetSystemLibrary.ExecuteConsoleCommand` "RH.SetSpeed 8" null)
  (`KismetSystemLibrary.Delay` 45.0)
  (`KismetSystemLibrary.PrintString` "STEP 3 - LIFE SUPPORT: building an Air Filtration Station ON floor -1 (underground = no shielding tax). Haulers bring Struct to the shaft head; the lift takes it down.")
  (`KismetSystemLibrary.ExecuteConsoleCommand` "RH.Build AirFilter 30 20 -1" null)
  (`KismetSystemLibrary.ExecuteConsoleCommand` "RH.SetSpeed 8" null)
  (`KismetSystemLibrary.Delay` 90.0)
  (`KismetSystemLibrary.ExecuteConsoleCommand` "RH.Habitat" null)
  (`KismetSystemLibrary.ExecuteConsoleCommand` "RH.SetSpeed 8" null)
  (`KismetSystemLibrary.Delay` 90.0)
  (`KismetSystemLibrary.PrintString` "STEP 4 - PRESSURIZE: the circulator pulls Oxygen from the colony pool down the trunk. 4 cells need 400 kg. Watch for the LIVABLE banner and the dot on the -1 cell.")
  (`KismetSystemLibrary.ExecuteConsoleCommand` "RH.Habitat" null)
  (`KismetSystemLibrary.ExecuteConsoleCommand` "RH.SetSpeed 8" null)
  (`KismetSystemLibrary.Delay` 120.0)
  (`KismetSystemLibrary.ExecuteConsoleCommand` "RH.Habitat" null)
  (`KismetSystemLibrary.PrintString` "VAULT DEMO DONE - if the exit banner has not fired yet, keep watching: the fill finishes within a minute or two. Click SURF / -1 on the SHAFT strip to ride the elevator yourself."))

(fn `UserConstructionScript`)